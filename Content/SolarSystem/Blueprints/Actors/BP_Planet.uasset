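; BP_Planet is a planet actor that continuously orbits the world origin in a circle on the XY plane.
; BeginPlay picks a small random starting angle between zero and one radian.
; Tick advances the angle by speed and delta time, then sets the location from its cosine and sine scaled by distance from the sun, without referencing a sun actor.
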(event `self.ReceiveBeginPlay`
  (set `self.f_Angle` (`KismetMathLibrary.RandomFloatInRange` 0.0 1.0)))

(event `self.ReceiveTick`
  (params (DeltaSeconds :type "Float (single-precision)"))
  (bind _output_get (set `self.f_Angle` (+ (`self.f_Angle`) (* DeltaSeconds (`self.f_MoveSpeed`)))))
  (`self.K2_SetActorLocation` (`KismetMathLibrary.MakeVector` (* (`KismetMathLibrary.Cos` _output_get) (`self.f_DistanceFromSun`)) (* (`KismetMathLibrary.Sin` _output_get) (`self.f_DistanceFromSun`)))))

(fn `UserConstructionScript`)