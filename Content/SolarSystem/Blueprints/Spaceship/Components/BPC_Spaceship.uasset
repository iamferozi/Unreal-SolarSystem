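; Spaceship component that simulates flight physics on the owner's skeletal mesh and exposes flight telemetry through GetInfo.
; Each tick it caches speed, pitch and center of mass, then applies thrust, lift and drag at that center.
; Working engines push forward by throttle; intact surfaces lift by capped horizontal speed squared times an angle-of-attack curve.
; Angle of attack comes from nose tilt against horizontal, not velocity, and drag coefficient scales with throttle.
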(event `self.ReceiveBeginPlay`
  (bind _spaceshipmesh (message `/Game/SolarSystem/Blueprints/Spaceship/Interface/BPI_SpaceShip.GetSpaceShipMesh` (`self.GetOwner`)))
  (set `self.Spaceship Mesh` _spaceshipmesh)
  (`self.CalculateMaxLiftForce`))

(event `self.ReceiveTick`
  (params (DeltaSeconds :type "Float (single-precision)"))
  (`|ExecutionSequence`
    (:`then_0`
      (`self.SetSpaceShipVariables`))
    (:`then_1`
      (`self.ApplyThrust`)
      (`self.CalculateAOA`)
      (`self.ApplyLift`)
      (`self.ApplyDrag`))))

(fn `ApplyDrag`
  (bind _returnvalue (* (* (* (`self.SpaceshipVelocity`) -1.0) (`KismetMathLibrary.MultiplyMultiply_FloatFloat` (`self.SpeedMPS`) 2.0)) (`KismetMathLibrary.Lerp` (`self.MinDragCoefficient`) (`self.MaxDragCoefficient`) (`self.Throttle`))))
  (set `self.DragForce` (`KismetMathLibrary.VSize` _returnvalue))
  (`PrimitiveComponent.AddForceAtLocation` (`self.Spaceship Mesh`) _returnvalue (`self.COM`) "None"))

(fn `ApplyLift`
  (`self.Spaceship Mesh`
    (:`then`
      (for _array_element (`self.Surfaces`)
        (bind (_surfaectype _surfacelocation _liftmultiplier _liftefficienycurve _b_surfacebroken) (break `/Game/SolarSystem/Blueprints/Spaceship/Data/Structures/Struct_SpaceSHipSurfaces` _array_element))
        (if (not _b_surfacebroken)
          (bind _liftforce (`self.CalculateLiftForce` _liftmultiplier _liftefficienycurve))
          (bind _returnvalue (* (`SceneComponent.GetUpVector` (`self.Spaceship Mesh`)) _liftforce))
          (set `self.LiftForce` (`KismetMathLibrary.VSize` _returnvalue))
          (`PrimitiveComponent.AddForceAtLocation` (`self.Spaceship Mesh`) _returnvalue (`self.COM`) "None"))))
    (:`else`)))

(fn `ApplyThrust`
  (`self.Spaceship Mesh`
    (:`then`
      (for _array_element (`self.Engines`)
        (bind (_acceleration _enginelocation _b_enginebroken _b_engineon) (break `/Game/SolarSystem/Blueprints/Spaceship/Data/Structures/Struct_SpaceshipEngine` _array_element))
        (if _b_engineon
          (if (not _b_enginebroken)
            (bind _thrustforce (`self.CalculateThrustForce` _acceleration))
            (bind _returnvalue (* (* (`SceneComponent.GetForwardVector` (`self.Spaceship Mesh`)) _thrustforce) (`self.Throttle`)))
            (set `self.ThrustForce` (`KismetMathLibrary.VSize` _returnvalue))
            (`PrimitiveComponent.AddForceAtLocation` (`self.Spaceship Mesh`) _returnvalue (`self.COM`) "None")))))
    (:`else`)))

(fn `CalculateAOA`
  (bind _spaceship_mesh (`self.Spaceship Mesh`)
    (:`then`
      (bind (_returnvalue_x _returnvalue_y) (`KismetMathLibrary.BreakVector` (`SceneComponent.GetForwardVector` _spaceship_mesh)))
      (bind _returnvalue (`KismetMathLibrary.DegAcos` (`KismetMathLibrary.Dot_VectorVector` (`SceneComponent.GetForwardVector` _spaceship_mesh) (`KismetMathLibrary.MakeVector` _returnvalue_x _returnvalue_y))))
      (set `self.AOA` (`KismetMathLibrary.SelectFloat` _returnvalue (* _returnvalue -1.0) (> (`self.Pitch`) 0.0))))
    (:`else`)))

(fn `CalculateLiftForce`
  (params (LiftMultiplier :type "Float (double-precision)") (LiftEfficiencyCurve :type "CurveFloat Object Reference"))
  (returns (LiftForce :type "Float (double-precision)"))
  (return (* (`KismetMathLibrary.FClamp` (* (/ (`KismetMathLibrary.MultiplyMultiply_FloatFloat` (`self.SpeedCMPS`) 2.0) 2.0) LiftMultiplier) 0.0 (`self.MaxLiftForce`)) (`CurveFloat.GetFloatValue` LiftEfficiencyCurve (`self.AOA`)))))

(fn `CalculateMaxLiftForce`
  (bind _spaceship_mesh (`self.Spaceship Mesh`)
    (:`then`
      (set `self.MaxLiftForce` (* (* (`PrimitiveComponent.GetMass` _spaceship_mesh) (`self.MaxLiftAcceleration`)) 100.0)))
    (:`else`)))

(fn `CalculateThrustForce`
  (params (Acceleration :type "Float (double-precision)"))
  (returns (ThrustForce :type "Float (double-precision)"))
  (return (* (* (`PrimitiveComponent.GetMass` (`self.Spaceship Mesh`)) Acceleration) 100.0)))

(fn `GetInfo`
  (returns (SpaceshipInfos :type "/Game/SolarSystem/Blueprints/Spaceship/Data/Structures/Struct_SpaceshipInfo Structure"))
  (return (make `/Game/SolarSystem/Blueprints/Spaceship/Data/Structures/Struct_SpaceshipInfo` (`self.SpaceshipAltitudeMPS`) (`self.AOA`) (`self.DragForce`) (`self.LiftForce`) (`self.Pitch`) (`self.SpeedCMPS`) (`self.SpeedMPS`) (`self.Throttle`) (`self.ThrustForce`))))

(fn `SetSpaceShipVariables`
  (bind (_returnvalue_roll _returnvalue_pitch) (`KismetMathLibrary.BreakRotator` (`SceneComponent.K2_GetComponentRotation` (`self.Spaceship Mesh`))))
  (bind _returnvalue (`SceneComponent.GetComponentVelocity` (`self.Spaceship Mesh`)))
  (bind (_returnvalue_x _returnvalue_y _returnvalue_z) (`KismetMathLibrary.BreakVector` (`SceneComponent.K2_GetComponentLocation` (`self.Spaceship Mesh`))))
  (`self.Spaceship Mesh`
    (:`then`
      (`|ExecutionSequence`
        (:`then_0`
          (set `self.COM` (`SkeletalMeshComponent.GetSkeletalCenterOfMass` (`self.Spaceship Mesh`)))
          (set `self.SpeedMPS` (/ (`KismetMathLibrary.VSizeXY` _returnvalue) 100.0))
          (set `self.SpaceshipVelocity` _returnvalue))
        (:`then_1`
          (set `self.Pitch` _returnvalue_pitch)
          (set `self.SpaceshipAltitudeMPS` (/ _returnvalue_z 100.0)))
        (:`then_2`
          (set `self.SpeedCMPS` (`KismetMathLibrary.VSizeXY` (`SceneComponent.GetComponentVelocity` (`self.Spaceship Mesh`)))))))
    (:`else`)))

(fn `SetThrottle`
  (params (ThrottleInput :type "Float (double-precision)"))
  (if (> ThrottleInput 0.0)
    (set `self.Throttle` (`KismetMathLibrary.FClamp` (+ (`self.Throttle`) (`self.ThrottleStep`))))
    (else
      (set `self.Throttle` (`KismetMathLibrary.FClamp` (- (`self.Throttle`) (`self.ThrottleStep`)))))))